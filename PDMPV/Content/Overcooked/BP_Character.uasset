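; Player character for an Overcooked-style game that moves via Enhanced Input and grabs, drops and interacts with objects.
; A short sphere trace ahead, on separate channels for grab and interact, finds targets and sends them interface messages.
; Grab attaches objects to Hands; grab input without a target drops them.
; SetIsInteracting toggles the interaction mapping context and blocks starting new interactions while active.
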(event Custom|Grab
  (params (ObjectToGrab :type BP%20Grabbable%20Object%20Reference))
  ;[1 1 1] ComentarioGrab Object To Actor
  (bind _output_get (Variables|Default|SetGrabedObject ObjectToGrab))
  (Transformation|AttachComponentToComponent _output_get (Variables|Default|GetHands) "None" "KeepWorld" "KeepWorld" "KeepWorld" true)
  (Components|MoveComponentTo (Variables|/Script/Engine.Actor|GetRootComponent (Variables|Default|GetGrabedObject)) "0, 0, 0" "0, 0, 0" false false 0.2 false))

(event Custom|SetIsInteracting
  (params (IsInteracting :type Boolean) (InteractingObject :type BPI%20Interactable%20Interface))
  (bind _returnvalue (Game|GetPlayerController 0))
  (bind _returnvalue_2 (PlayerController|LocalPlayerSubsystems|GetEnhancedInputLocalPlayerSubsystem _returnvalue))
  (Variables|Default|SetIsInteracting IsInteracting)
  (Variables|Default|SetInteracting%20Object InteractingObject)
  (if (Variables|Default|GetIsInteracting)
    (Input|AddMappingContext _returnvalue_2 "/Game/Inputs/IMC_Interaction.IMC_Interaction" 0 "(bIgnoreAllPressedKeysUntilRelease=True,bForceImmediately=False,bNotifyUserSettings=False)")
    (else
      (Input|RemoveMappingContext _returnvalue_2 "/Game/Inputs/IMC_Interaction.IMC_Interaction" "(bIgnoreAllPressedKeysUntilRelease=True,bForceImmediately=False,bNotifyUserSettings=False)"))))

(event Input|EnhancedActionEvents|EnhancedInputActionIA_Movement
  (params (ActionValue :type Vector%202D%20Structure) (ElapsedSeconds :type Float%20%28double-precision%29) (TriggeredSeconds :type Float%20%28double-precision%29) (InputAction :type Input%20Action%20Object%20Reference :default "/Game/Inputs/IA_Movement.IA_Movement"))
  ;[1 1 1] Character Input Movement
  (Pawn|Input|AddMovementInput (Math|Conversions|ToVector(Vector2D) ActionValue) 1.0 false))

(event Input|EnhancedActionEvents|EnhancedInputActionIA_GrabDrop
  (params (ActionValue :type Boolean) (ElapsedSeconds :type Float%20%28double-precision%29) (TriggeredSeconds :type Float%20%28double-precision%29) (InputAction :type Input%20Action%20Object%20Reference :default "/Game/Inputs/IA_GrabDrop.IA_GrabDrop"))
  (bind (_returnvalue _grabedobject) (CallFunction|GetGrabbedObject))
  ;[0.003805 1 0.008206] Character Interaction
  (:Started
    (bind (_returnvalue_2 _outhit) (CallFunction|FindObjecttoInteractwith "TraceTypeQuery3"))
    (if _returnvalue_2
      (Class|BPIInteractable|GrabDrop(Message) (.HitActor (Collision|BreakHitResult _outhit)) self)
      (elif _returnvalue
        (Default|Drop _grabedobject)
        (Variables|Default|SetGrabedObject 0)))))

(event Input|EnhancedActionEvents|EnhancedInputActionIA_StartInteract
  (params (ActionValue :type Boolean) (ElapsedSeconds :type Float%20%28double-precision%29) (TriggeredSeconds :type Float%20%28double-precision%29) (InputAction :type Input%20Action%20Object%20Reference :default "/Game/Inputs/IA_StartInteract.IA_StartInteract"))
  (:Started
    (if (not (Variables|Default|GetIsInteracting))
      (bind (_returnvalue _outhit) (CallFunction|FindObjecttoInteractwith "TraceTypeQuery1"))
      (if _returnvalue
        (Class|BPIInteractable|Interact(Message) (.HitActor (Collision|BreakHitResult _outhit)) self)))))

(event EventBeginPlay)

(event Collision|EventActorBeginOverlap
  (params (OtherActor :type Actor%20Object%20Reference)))

(fn ConstructionScript)

(fn GetGrabbedObject
  (bind _grabedobject (Variables|Default|GetGrabedObject))
  (return (Utilities|IsValid _grabedobject) _grabedobject))

(fn FindObjecttoInteractwith
  (params (TraceChannel :type ETraceTypeQuery%20Enum :default "TraceTypeQuery1"))
  (bind _returnvalue (Transformation|GetActorForwardVector))
  (bind _returnvalue_2 (Transformation|GetActorLocation))
  (bind _returnvalue_3 (* _returnvalue 5e+01))
  (bind _returnvalue_4 (+ _returnvalue_3 _returnvalue_2))
  (bind (_x _y _z) (Math|Vector|BreakVector _returnvalue_4))
  (bind (_outhit _returnvalue_5) (Collision|SphereTraceByChannel (Math|Vector|MakeVector _x _y (+ _z -5e+01)) (Math|Vector|MakeVector _x _y (+ _z 1e+01)) 3e+01 TraceChannel false (Utilities|Array|MakeArray (Variables|Default|GetGrabedObject)) "ForDuration"))
  (return _returnvalue_5 _outhit))