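; Kitchen table interactable with a slicing station, where a player works on food items placed on it.
; Interact accepts only a sliceable BP_FoodItem, sets its state, records the player and flags the table as interacting.
; GrabDrop defers to the parent only when Progress is 0 or 1, then resets it; this graph never advances Progress.
; Both Interact and StopInteraction pass false to the player's SetIsInteracting.
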(event EventBeginPlay
  (|CallParentFunction) ; Este nodo está deshabilitado y no se le llamará.\nArrastra pines para construir una funcionalidad.
)

(event Collision|EventActorBeginOverlap
  (params (OtherActor :type Actor%20Object%20Reference))
  (|CallParentFunction OtherActor) ; Este nodo está deshabilitado y no se le llamará.\nArrastra pines para construir una funcionalidad.
)

(event EventTick
  (params (DeltaSeconds :type Float%20%28single-precision%29))
  (|CallParentFunction DeltaSeconds) ; Este nodo está deshabilitado y no se le llamará.\nArrastra pines para construir una funcionalidad.
)

(event EventGrabDrop
  (params (Player :type BP%20Character%20Object%20Reference))
  (if (CallFunction|CanGrabObject)
    (|CallParentFunction Player)
    (Variables|Default|SetProgress 0.0)))

(event EventInteract
  (params (Player :type BP%20Character%20Object%20Reference))
  (bind _asbp_food_item (Utilities|Casting|CastToBP_FoodItem (Variables|Default|GetPlaceTarget)))
  (if (Default|CanbeSliced _asbp_food_item)
    (Default|SetState _asbp_food_item "NewEnumerator0")
    (Default|SetIsInteracting Player false _asbp_food_item)
    (Variables|Default|SetInteractingPlayer Player)
    (Variables|Default|SetIsInteracting true)))

(event EventStopInteraction
  (Variables|Default|SetIsInteracting false)
  (Default|SetIsInteracting (Variables|Default|GetInteractingPlayer) false))

(fn ConstructionScript
  (|CallParentFunction))

(fn CanGrabObject
  (return (or (== (Variables|Default|GetProgress) 0.0) (== (Variables|Default|GetProgress) 1.0))))