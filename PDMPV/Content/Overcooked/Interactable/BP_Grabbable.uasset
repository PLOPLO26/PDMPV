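; BP_Grabbable is an interactable physics object that a player can pick up and drop in the Overcooked game.
; GrabDrop picks it up only if the player holds nothing, turning off mesh physics and collision before passing itself to the player's Grab.
; Drop detaches it in world space and restores physics and collision, but GrabDrop never calls it.
; Interact and StopInteraction are empty.
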(event Custom|Drop
  (bind _mesh (Variables|Default|GetMesh))
  ;[0.135 0.5127 1] Detach From Actor
  (Transformation|DetachFromActor "KeepWorld" "KeepWorld" "KeepWorld")
  (Physics|SetSimulatePhysics _mesh true)
  (Collision|SetCollisionEnabled _mesh "QueryAndPhysics"))

(event Custom|Grab
  (params (Player :type BP%20Character%20Object%20Reference))
  (bind _mesh (Variables|Default|GetMesh))
  (Physics|SetSimulatePhysics _mesh false)
  (Collision|SetCollisionEnabled _mesh "NoCollision")
  (Default|Grab Player self))

(event EventBeginPlay)

(event Collision|EventActorBeginOverlap
  (params (OtherActor :type Actor%20Object%20Reference)))

(event EventTick
  (params (DeltaSeconds :type Float%20%28single-precision%29)))

(event EventStopInteraction)

(event EventInteract
  (params (Player :type BP%20Character%20Object%20Reference)))

(event EventGrabDrop
  (params (Player :type BP%20Character%20Object%20Reference))
  ;[1 0.8905 0.1445] Interaction
  (if (CallFunction|CanbeGrabed Player)
    (CallFunction|Grab Player)))

(fn ConstructionScript)

(fn CanbeGrabed
  (params (Player :type BP%20Character%20Object%20Reference))
  (return (not (.ReturnValue (Default|GetGrabbedObject Player)))))