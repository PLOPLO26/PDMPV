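; BP_Table is an interactable table for an Overcooked-style game that holds one object for the player to place or pick up.
; GrabDrop moves the player's held object onto a free table, attaching it with world transforms kept, then calling MoveComponentTo on its root.
; An empty-handed player takes the stored PlaceTarget back through Grab, freeing the table.
; Interact is empty, and no logic runs on Tick.
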(event EventBeginPlay)

(event Collision|EventActorBeginOverlap
  (params (OtherActor :type Actor%20Object%20Reference)))

(event EventTick
  (params (DeltaSeconds :type Float%20%28single-precision%29)))

(event EventGrabDrop
  (params (Player :type BP%20Character%20Object%20Reference))
  (bind (_returnvalue _grabedobject) (Default|GetGrabbedObject Player))
  (if _returnvalue
    (Utilities|IsValid (Variables|Default|GetPlaceTarget)
      (:Is%20Not%20Valid
        (bind _output_get (Variables|Default|SetPlaceTarget _grabedobject))
        (Transformation|AttachComponentToComponent _output_get (Variables|Default|GetTarget) "None" "KeepWorld" "KeepWorld" "KeepWorld" true)
        (Components|MoveComponentTo (Variables|/Script/Engine.Actor|GetRootComponent (Variables|Default|GetPlaceTarget)) "0, 0, 0" "0, 0, 0" false false 0.2 false)
        (Variables|/Game/Overcooked/BP_Character.BP_Character_C|SetGrabedObject Player 0)))
    (else
      ;[0.3876 0.4015 1] Grab The Object from the table
      (Utilities|IsValid (Variables|Default|GetPlaceTarget)
        (:Is%20Valid
          (Default|Grab Player (Variables|Default|GetPlaceTarget))
          (Variables|Default|SetPlaceTarget 0))))))

(event EventInteract
  (params (Player :type BP%20Character%20Object%20Reference)))

(fn ConstructionScript)