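; BP_FoodItem is an interactable food ingredient in an Overcooked-style game, with Raw, Slicing and Sliced states.
; It begins play as Raw, and its SetState event stores the new state and swaps the mesh material to match.
; CanBeSliced returns the IsSlicable flag.
; CanBeGrabed allows a grab only when the player's grabbed object is a BP_Dish with free space.
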(event Custom|SetState
  (params (Sate :type BPE_FoodItemStates%20Enum :default "NewEnumerator0"))
  (bind _output_get (Variables|Default|SetSate Sate))
  (Rendering|Material|SetMaterial (Variables|Character|GetMesh) 0 (Utilities|Select :Index _output_get :NewEnumerator0 "/Game/Materiales/BaseColor/M_Raw.M_Raw" :NewEnumerator1 "/Game/Materiales/BaseColor/M_Slicing.M_Slicing" :NewEnumerator2 "/Game/Materiales/BaseColor/M_Sliced.M_Sliced")))

(event EventBeginPlay
  (CallFunction|SetState "NewEnumerator0"))

(event Collision|EventActorBeginOverlap
  (params (OtherActor :type Actor%20Object%20Reference))
  (|CallParentFunction OtherActor) ; Este nodo está deshabilitado y no se le llamará.\nArrastra pines para construir una funcionalidad.
)

(event EventTick
  (params (DeltaSeconds :type Float%20%28single-precision%29))
  (|CallParentFunction DeltaSeconds) ; Este nodo está deshabilitado y no se le llamará.\nArrastra pines para construir una funcionalidad.
)

(fn ConstructionScript
  (|CallParentFunction))

(fn CanbeSliced
  (return (Variables|Default|GetIsSlicable)))

(fn CanbeGrabed
  (params (Player :type BP%20Character%20Object%20Reference))
  (bind (_returnvalue _grabedobject) (Default|GetGrabbedObject Player))
  (if (not _returnvalue)
    (return false)
    (else
      (bind _asbp_dish (Utilities|Casting|CastToBP_Dish _grabedobject)
        (:then
          (return (Default|HasPlace _asbp_dish)))
        (:CastFailed
          (return false))))))