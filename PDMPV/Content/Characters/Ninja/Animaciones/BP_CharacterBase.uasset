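; Base character Blueprint, stored with the Ninja animations, that provides health and damage handling.
; RecibirDaño subtracts the incoming amount from Vida and clamps the result to a fixed range.
; At zero health it only prints a death message; otherwise it prints the damage received and plays the MontageDaño hit montage.
; The event graph and construction script hold no active logic, so damage depends on calls to that function.
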(event EventBeginPlay)

(event Collision|EventActorBeginOverlap
  (params (OtherActor :type Actor%20Object%20Reference)))

(event EventTick
  (params (DeltaSeconds :type Float%20%28single-precision%29)))

(fn ConstructionScript)

(fn RecibirDaño
  (params (Cantidad :type Float%20%28double-precision%29))
  (bind _output_get (Variables|Default|SetVida (Math|Float|Clamp(Float) (- (Variables|Default|GetVida) Cantidad) 0.0 1e+02)))
  (if (<= _output_get 0.0)
    (Development|PrintText "MUERTO" true true "(R=0.889583,G=0.000000,B=0.036676,A=1.000000)")
    (else
      (Development|PrintText (Utilities|Text|ToText(String) (Utilities|String|Append "Daño Recibido" (Utilities|String|ToString(Float) Cantidad))) true true "(R=1.000000,G=0.000000,B=0.016606,A=1.000000)")
      (Animation|PlayAnimMontage (Variables|Default|Get%20Montage%20Daño) 1.0 "None"))))